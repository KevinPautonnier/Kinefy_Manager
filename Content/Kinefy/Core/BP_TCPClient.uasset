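; BP_TCPClient is the Kinefy TCP client actor that connects to a server on the local network and sends it atelier launch commands.
; Launchconnection builds a 192.168.x.y address from two parts and connects on a fixed port.
; Received slash-delimited messages prefixed "kinefy" store the remainder as ServerIP and call ServerFound.
; LaunchAtelier emits an "atelier/<number>" string as bytes over the socket.
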(event OnReceivedBytes(TCPClient)
  (params (Bytes :type Array%20of%20Bytes))
  (bind _returnvalue (Class|CustomDeserialize|CustomBytestoString Bytes))
  (bind (_lefts _rights) (Utilities|String|Split _returnvalue "/"))
  (if (Utilities|Enum|Equal(Enum) _lefts "kinefy")
    (Variables|Default|SetServerIP _rights)
    (Development|PrintString _rights)
    (Default|CallServerFound)))

(event Custom|Launch%20connection
  (params (IPFirstPart :type String) (IPSecondPart :type String))
  (bind _returnvalue (Utilities|String|Append "192.168." IPFirstPart "." IPSecondPart))
  (Class|TCPClientComponent|ConnecttoSocketasClient (Variables|Default|GetTCPClient) _returnvalue 7000)
  (Development|PrintString _returnvalue))

(event Custom|LaunchAtelier
  (params (InInt :type Integer))
  (Class|TCPClientComponent|Emit (Variables|Default|GetTCPClient) (Class|CustomSerialize|CustomStringtoBytes (Utilities|String|Append "atelier/" (Utilities|String|ToString(Integer) InInt)))))

(fn ConstructionScript)