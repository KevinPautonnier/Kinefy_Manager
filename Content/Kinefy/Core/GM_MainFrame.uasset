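; Game mode for the Kinefy main frame, bridging the main UI widget and a TCP client.
; On BeginPlay it shows WBP_MainFrame, spawns BP_TCPClient, binds to its server-found event and enables the mouse cursor with game-and-UI input.
; It forwards connection requests with a two-part IP and atelier launches to the client, and its ServerFound event tells the widget to show the ateliers.
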(event Custom|LaunchConnection
  (params (IPFirstPart :type String) (IPSecondPart :type String))
  (Default|LaunchConnection (Variables|Default|GetAsTCPClient) IPFirstPart IPSecondPart))

(event Custom|ServerFound
  (Default|ShowAteliers (Variables|Default|GetAsMainFrame)))

(event Custom|TCPLaunchAtelier
  (params (InInt :type Integer))
  (Default|LaunchAtelier (Variables|Default|GetAsTCPClient) InInt))

(event EventBeginPlay
  (bind _returnvalue (Game|GetPlayerController 0))
  (bind _returnvalue_2 (UserInterface|CreateWidget "/Game/Kinefy/UI/Core/WBP_MainFrame.WBP_MainFrame_C"))
  (bind _output_get (Variables|Default|SetAsMainFrame _returnvalue_2))
  (UserInterface|Viewport|AddtoViewport _output_get 0)
  (bind _returnvalue_3 (Game|SpawnActorfromClass "/Game/Kinefy/Core/BP_TCPClient.BP_TCPClient_C" (Math|Transform|MakeTransform "0, 0, 0" "0, 0, 0" "1.000000,1.000000,1.000000") "Undefined" 0 0))
  (bind _output_get_2 (Variables|Default|SetAsTCPClient _returnvalue_3))
  (EventDispatchers|BindEventtoServerFound _output_get_2 (EventDispatchers|CreateEvent :!event Custom|ServerFound))
  (Input|SetInputModeGameandUI _returnvalue 0 "DoNotLock" true)
  (Variables|/Script/Engine.PlayerController|SetbShowMouseCursor _returnvalue true))

(fn ConstructionScript)